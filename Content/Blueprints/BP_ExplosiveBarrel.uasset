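; BP_ExplosiveBarrel is a destructible barrel that explodes once incoming damage depletes its health.
; Its AnyDamage event lowers health, then a one-time flag guards the radial damage, which reuses the final hit's damage amount and ignores the barrel itself.
; The blast spawns a rocket launcher explosion effect scaled to the radius, plays a sound and destroys the actor.
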(event `self.ReceiveBeginPlay`
  ;[1 1 1] Ignore Damage To Self
  (set `self.Ignore Actors` (`|MakeArray` self :!type "Actor Object Reference")))

(event `self.ReceiveAnyDamage`
  (params (Damage :type "Float (single-precision)") (DamageType :type "DamageType Object Reference") (InstigatedBy :type "Controller Object Reference") (DamageCauser :type "Actor Object Reference"))
  (bind _returnvalue (`self.K2_GetActorLocation`))
  (bind _explosion_radius (`self.Explosion Radius`))
  ;[1 1 1] If taken enough damage, explode
  (if (not (`self.exploded`))
    (bind _output_get (set `self.Health` (- (`self.Health`) Damage)))
    (if (<= _output_get 0.0)
      (set `self.exploded` true)
      (`GameplayStatics.ApplyRadialDamage` (`self.Damage`) _returnvalue _explosion_radius null (`self.Ignore Actors`) null null (`self.Do Full Damage`))
      (`GameplayStatics.SpawnEmitterAtLocation` "/Game/PrototypeWeap/FX/P_RocketLauncher_Explosion.P_RocketLauncher_Explosion" _returnvalue (struct) (`KismetMathLibrary.Conv_DoubleToVector` (/ _explosion_radius 120.0)))
      (`GameplayStatics.PlaySoundAtLocation` "/Game/PrototypeWeap/Sound/RocketLauncher/RL_Explosion_Cue.RL_Explosion_Cue" _returnvalue (struct) 1.0 1.0 0.0 null null null null)
      (`self.K2_DestroyActor`))))

(fn `UserConstructionScript`)