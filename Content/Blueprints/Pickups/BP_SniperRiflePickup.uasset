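; Sniper rifle pickup that the player collects by walking into its trigger.
; On overlap with BP_Player it adds sniper reserve ammo, flags the sniper rifle as held and clears the rocket launcher flag.
; It swaps the visibility of the player's two weapon components, plays an ammo pickup sound at its location and destroys itself.
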(event `self.PickupTrigger.OnComponentBeginOverlap`
  (params (OverlappedComponent :type "PrimitiveComponent Object Reference") (OtherActor :type "Actor Object Reference") (OtherComp :type "PrimitiveComponent Object Reference") (OtherBodyIndex :type Integer) (bFromSweep :type Boolean) (SweepResult :type "HitResult Structure (by ref)"))
  (bind _asbp_player (cast `/Game/Blueprints/BP_Player` OtherActor))
  (set `/Game/Blueprints/BP_Player.SniperReserveAmmo` (+ (`/Game/Blueprints/BP_Player.SniperReserveAmmo` _asbp_player) 5) _asbp_player)
  (set `/Game/Blueprints/BP_Player.HasSniperRifle?` true _asbp_player)
  (set `/Game/Blueprints/BP_Player.HasRocketLauncher?` false _asbp_player)
  (`GameplayStatics.PlaySoundAtLocation` "/Game/PrototypeWeap/Sound/SniperRifle/SR_AmmoPickup01_Cue.SR_AmmoPickup01_Cue" (`self.K2_GetActorLocation`) (struct) 1.0 1.0 0.0 null null null null)
  (`SceneComponent.SetVisibility` (`/Game/Blueprints/BP_Player.SniperRifle` _asbp_player) true false)
  (`SceneComponent.SetVisibility` (`/Game/Blueprints/BP_Player.RocketLauncher` _asbp_player) false false)
  (`self.K2_DestroyActor`))

(fn `UserConstructionScript`)