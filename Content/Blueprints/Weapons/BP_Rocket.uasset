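; Rocket projectile that flies forward and explodes on overlap or after a timeout.
; Tick moves it along its forward vector by Speed each frame, unscaled by delta time and without sweeping.
; Sphere overlap sets Colliding after a BP_Player class check on the overlapped component, triggering Explode next tick.
; Explode applies radial damage, radius-scaled particles, sound, AI noise and a debug sphere, then stops the flight sound and destroys the actor.
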(event `self.ReceiveTick`
  (params (DeltaSeconds :type "Float (single-precision)"))
  (bind _returnvalue (`self.K2_GetActorLocation`))
  ;[1 1 1] Rocket Fly Loop, explode on collide, destroy if active for too long
  (if (`self.Colliding`)
    (`self.Explode`)
    (else
      (`self.K2_SetActorLocation` (`KismetMathLibrary.VLerp` _returnvalue (+ _returnvalue (* (`self.GetActorForwardVector`) 1.0)) (`self.Speed`)))
      (bind _output_get (set `self.Timeout_Counter` (+ (`self.Timeout_Counter`) DeltaSeconds)))
      (if (> _output_get (`self.Timeout`))
        (`self.Explode`)))))

(event `Explode`
  (bind _returnvalue (`self.K2_GetActorLocation`))
  (bind _explosion_radius (`self.Explosion Radius`))
  ;[1 1 1] Explode Rocket
  (`GameplayStatics.PlaySoundAtLocation` "/Game/PrototypeWeap/Sound/RocketLauncher/RL_Explosion_Cue.RL_Explosion_Cue" _returnvalue (struct) 1.0 1.0 0.0 null null null null)
  (`GameplayStatics.ApplyRadialDamage` :`BaseDamage` (`self.Damage`) :`Origin` _returnvalue :`DamageRadius` _explosion_radius :`DamageCauser` self :`InstigatedByController` null)
  (`GameplayStatics.SpawnEmitterAtLocation` "/Game/PrototypeWeap/FX/P_RocketLauncher_Explosion.P_RocketLauncher_Explosion" _returnvalue (struct) (`KismetMathLibrary.Conv_DoubleToVector` (/ _explosion_radius 120.0)))
  (`AISense_Hearing.ReportNoiseEvent` _returnvalue 20.0 null)
  (`KismetSystemLibrary.DrawDebugSphere` _returnvalue _explosion_radius 60 (struct :`R` 1.0 :`B` 0.083664 :`A` 1.0) 3.0 1.0)
  (`AudioComponent.Stop` (`self.InAirSound`))
  (`self.K2_DestroyActor`))

(event `self.ReceiveBeginPlay`
  ;[1 1 1] Setup sound
  (bind _returnvalue (`GameplayStatics.CreateSound2D` "/Game/PrototypeWeap/Sound/RocketLauncher/RL_InAirLoop_Cue.RL_InAirLoop_Cue" 1.0 1.0 0.0 null))
  (bind _output_get (set `self.InAirSound` _returnvalue))
  (`AudioComponent.Play` _output_get 0.0))

(event `self.Sphere.OnComponentBeginOverlap`
  (params (OverlappedComponent :type "PrimitiveComponent Object Reference") (OtherActor :type "Actor Object Reference") (OtherComp :type "PrimitiveComponent Object Reference") (OtherBodyIndex :type Integer) (bFromSweep :type Boolean) (SweepResult :type "HitResult Structure (by ref)"))
  (if (not (`KismetMathLibrary.ClassIsChildOf` (`GameplayStatics.GetObjectClass` OverlappedComponent) "/Game/Blueprints/BP_Player.BP_Player_C"))
    (set `self.Colliding` true)))

(fn `UserConstructionScript`)